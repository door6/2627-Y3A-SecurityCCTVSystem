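; BP_Springtrapp is an AI-driven Springtrap character that pursues the player.
; On BeginPlay it sets walk speed and animation rate, waits, teleports to a hard-coded location and starts MoveTowardsPlayer.
; That event runs AIMoveTo on the player, retrying after a short delay on failure but ending after a delay on success.
; A check for the player moving outside their room radius is disconnected and never runs.
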(event `self.ReceiveBeginPlay`
  (set `CharacterMovementComponent.MaxWalkSpeed` 200.0 (`self.CharacterMovement`))
  (`SkeletalMeshComponent.SetPlayRate` (`self.Mesh`) 1.5)
  (`KismetSystemLibrary.Delay` 5.0)
  (`self.K2_SetActorLocation` (3640.0 -5780.0 228.0))
  (`self.MoveTowardsPlayer`))

(event `self.ReceiveTick`
  (params (DeltaSeconds :type "Float (single-precision)")))

(event `MoveTowardsPlayer`
  (`|AIMoveTo` self (0.0 0.0 0.0) (`GameplayStatics.GetPlayerCharacter` 0) 10.0 :!label _label
    (:`OnSuccess`
      (`KismetSystemLibrary.Delay` 2.0))
    (:`OnFail`
      (`KismetSystemLibrary.Delay` 0.2)
      (goto _label))))

(fn `UserConstructionScript`
  (`parent.UserConstructionScript`))