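; BP_Light is a light actor that changes color with the security state, switching between neutral and alarm looks.
; On BeginPlay it sets the PointLight to the neutral color and creates a dynamic material on the Sphere mesh with a matching emissive color.
; A Responder component's OnRespondTriggered event switches both the light color and the EmissiveFactor parameter to the neutral or alarm color.
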(event `self.ReceiveBeginPlay`
  (bind _neutralcolor (`self.NeutralColor`))
  (`LightComponent.SetLightColor` (`self.PointLight`) _neutralcolor true)
  (bind _returnvalue (`PrimitiveComponent.CreateDynamicMaterialInstance` (`self.Sphere`) 0 "/Game/Assets/scene/Materials/light.light" "dynamic_light"))
  (bind _output_get (set `self.DynamicMaterial` _returnvalue))
  (`MaterialInstanceDynamic.SetVectorParameterValue` _returnvalue "EmissiveFactor" _neutralcolor)
  (`MaterialInstanceDynamic.SetVectorParameterValue` _output_get "EmissiveFactor" _neutralcolor))

(event `self.Responder.OnRespondTriggered`
  (params (SecurityState :type "ESecurityState Enum" :default "Neutral"))
  (switch `ESecurityState` SecurityState
    (:`Neutral`
      (`LightComponent.SetLightColor` (`self.PointLight`) (`self.NeutralColor`) true)
      (`MaterialInstanceDynamic.SetVectorParameterValue` (`self.DynamicMaterial`) "EmissiveFactor" (`self.NeutralColor`)))
    (:`Alarm`
      (`LightComponent.SetLightColor` (`self.PointLight`) (`self.AlarmColor`) true)
      (`MaterialInstanceDynamic.SetVectorParameterValue` (`self.DynamicMaterial`) "EmissiveFactor" (`self.AlarmColor`)))))

(fn `UserConstructionScript`)