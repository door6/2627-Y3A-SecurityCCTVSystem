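; BP_Intruder is an AI-moved pawn that travels a one-way route through three hard-coded world locations when play begins.
; BeginPlay chains AIMoveTo calls, pausing briefly after reaching each of the first two points.
; A failed move retries the same point after a short delay, and the route ends at the third point without looping.
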(event `self.ReceiveBeginPlay`
  (`|AIMoveTo` self (240.0 630.0 90.0) null 200.0 :!label _label
    (:`OnSuccess`
      (`KismetSystemLibrary.Delay` 2.0)
      (`|AIMoveTo` self (-790.0 430.0 40.0) null 200.0 :!label _label_2
        (:`OnSuccess`
          (`KismetSystemLibrary.Delay` 2.0)
          (`|AIMoveTo` self (-920.0 -390.0 100.0) null 100.0 :!label _label_3
            (:`OnFail`
              (`KismetSystemLibrary.Delay` 0.2)
              (goto _label_3))))
        (:`OnFail`
          (`KismetSystemLibrary.Delay` 0.2)
          (goto _label_2))))
    (:`OnFail`
      (`KismetSystemLibrary.Delay` 0.2)
      (goto _label))))

(fn `UserConstructionScript`)