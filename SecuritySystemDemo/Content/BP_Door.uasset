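; BP_Door is a door that swings between its starting rotation and an alarm rotation when its Responder reports a security state change.
; BeginPlay derives a hinge pivot from the mesh bounds, using the longer horizontal extent, and stores both target rotations.
; Each response picks a target and flips the rotation speed's sign.
; Tick orbits the actor around the pivot while yawing it until it nears the target within a tolerance.
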(event `self.ReceiveBeginPlay`
  (bind _returnvalue (`self.K2_GetActorRotation`))
  (bind _staticmesh (`self.StaticMesh`))
  (bind (_origin _boxextent) (`KismetMathLibrary.BreakBoxSphereBounds` (`StaticMesh.GetBounds` (`StaticMeshComponent.StaticMesh` _staticmesh))))
  (set `self.PivotLocation` (`KismetMathLibrary.TransformLocation` (`SceneComponent.K2_GetComponentToWorld` _staticmesh) (- _origin (`KismetMathLibrary.SelectVector` (`KismetMathLibrary.MakeVector` (.x _boxextent)) (`KismetMathLibrary.MakeVector` 0.0 (.y _boxextent)) (> (.x _boxextent) (.y _boxextent))))))
  (bind _output_get (set `self.NeutralRotation` _returnvalue))
  (set `self.TargetRotation` _output_get)
  (set `self.AlarmRotation` (`KismetMathLibrary.MakeRotator` 0.0 0.0 (- (.yaw _returnvalue) (`self.MaxRotation`)))))

(event `self.ReceiveTick`
  (params (DeltaSeconds :type "Float (single-precision)"))
  (`self.PlayDoorAnimation`))

(event `self.Responder.OnRespondTriggered`
  (params (SecurityState :type "ESecurityState Enum" :default "Neutral"))
  (switch `ESecurityState` SecurityState
    (:`Neutral`
      (set `self.TargetRotation` (`self.NeutralRotation`)))
    (:`Alarm`
      (set `self.TargetRotation` (`self.AlarmRotation`))))
  (set `self.RotationSpeed` (* (`self.RotationSpeed`) -1.0))
  (set `self.IsDoorMoving` true))

(event `PlayDoorAnimation`
  (bind _returnvalue (* (`GameplayStatics.GetWorldDeltaSeconds`) (`self.RotationSpeed`)))
  (if (`self.IsDoorMoving`)
    (if (!= (`self.K2_GetActorRotation`) (`self.TargetRotation`) :`ErrorTolerance` 0.8)
      (`self.K2_SetActorLocation` (+ (`self.PivotLocation`) (`KismetMathLibrary.RotateAngleAxis` (- (`self.K2_GetActorLocation`) (`self.PivotLocation`)) _returnvalue (0.0 0.0 1.0))))
      (`self.K2_AddActorWorldRotation` (`KismetMathLibrary.MakeRotator` 0.0 0.0 _returnvalue))
      (else
        (set `self.IsDoorMoving` false)))))

(fn `UserConstructionScript`)